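; Player controller Blueprint for mouse-driven placement of roots on a grid, creating the WB_UI widget on BeginPlay.
; Each tick a cursor trace snaps a preview BP_Root to the nearest visible GridManager cell.
; Left click spawns a root there if placement is valid and registers it with the cell.
; Water and Mineral counters key off SpawnRoot's result, but its return node is unwired, as is the cursor/input-mode setup.
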(event `self.ReceiveBeginPlay`
  (`self.Set Placement Enabled` true)
  (bind _returnvalue (`|CreateWidget` "/Game/Assets/Blueprints/Gamemode/WB_UI.WB_UI_C"))
  (`UserWidget.AddToViewport` _returnvalue 0))

(event `self.ReceiveTick`
  (params (DeltaSeconds :type "Float (single-precision)"))
  (`self.UpdatePlacement`))

(event `Key|LeftMouseButton`
  (params (Key :type "Key Structure"))
  (:`Pressed`
    (bind _type (`self.SpawnRoot`))
    (`KismetSystemLibrary.PrintString` (`|GetEnumeratorNameAsString` _type))
    (switch `/Game/Assets/Type` _type
      (:`NewEnumerator1`
        (bind _output_get (set `/Game/Assets/Blueprints/Gamemode/WB_UI.WaterCount` (+ (`/Game/Assets/Blueprints/Gamemode/WB_UI.WaterCount` (stale `self.ReceiveBeginPlay` _returnvalue)) 1) (stale `self.ReceiveBeginPlay` _returnvalue)))
        (`KismetSystemLibrary.PrintText` (`KismetTextLibrary.Conv_IntToText` _output_get)))
      (:`NewEnumerator5`
        (bind _output_get_2 (set `/Game/Assets/Blueprints/Gamemode/WB_UI.MineralCount` (+ (`/Game/Assets/Blueprints/Gamemode/WB_UI.MineralCount` (stale `self.ReceiveBeginPlay` _returnvalue)) 1) (stale `self.ReceiveBeginPlay` _returnvalue)))
        (`KismetSystemLibrary.PrintText` (`KismetTextLibrary.Conv_IntToText` _output_get_2))))))

(fn `Set Placement Enabled`
  (params (isEnabled :type Boolean))
  (bind _placebleactor (`self.PlacebleActor`))
  (if (== isEnabled (`self.PlacementEnabled`))
    (return)
    (else
      (bind _output_get (set `self.PlacementEnabled` isEnabled))
      (if _output_get
        (bind _returnvalue (`|SpawnActorFromClass` "/Game/Assets/Blueprints/BP_Root.BP_Root_C" (`KismetMathLibrary.MakeTransform` (0.0 20.0 0.0)) "AlwaysSpawn" "OverrideRootScale" null null))
        (bind _output_get_2 (set `self.PlacebleActor` _returnvalue))
        (bind _returnvalue_2 (`self.GetComponentByClass` _output_get_2 "/Game/Assets/Blueprints/Component/AC_Clickable.AC_Clickable_C"))
        (`/Engine/EditorBlueprintResources/StandardMacros.IsValid` _returnvalue_2
          (:`Is Valid`
            (`/Game/Assets/Blueprints/Component/AC_Clickable.InPlacement` _returnvalue_2))
          (:`Is Not Valid`
            _))
        (`AddComponent|NODE_AddAC_PlacableCopmponent-0` :`self` _output_get_2)
        (else
          (`/Engine/EditorBlueprintResources/StandardMacros.IsValid` _placebleactor
            (:`Is Valid`
              (`self.K2_DestroyActor` _placebleactor))))))))

(fn `SpawnRoot`
  (returns (Type :type "/Game/Assets/Type Enum"))
  (bind _placebleactor (`self.PlacebleActor`))
  (bind _returnvalue (`self.GetComponentByClass` _placebleactor "/Game/Assets/Blueprints/Component/AC_PlacableCopmponent.AC_PlacableCopmponent_C"))
  (`/Engine/EditorBlueprintResources/StandardMacros.IsValid` _returnvalue
    (:`Is Valid`
      (if (`/Game/Assets/Blueprints/Component/AC_PlacableCopmponent.isPlacementValid` _returnvalue)
        (bind _returnvalue_2 (`|SpawnActorFromClass` "/Game/Assets/Blueprints/BP_Root.BP_Root_C" (`self.GetTransform` _placebleactor) "AlwaysSpawn" "OverrideRootScale" null null))
        (bind _returnvalue_3 (`GameplayStatics.GetActorOfClass` "/Game/Assets/Blueprints/Gamemode/GridManager.GridManager_C"))
        (bind _outputgridcell (`/Game/Assets/Blueprints/Gamemode/GridManager.GetClosestGridCell` _returnvalue_3 (`self.K2_GetActorLocation` _placebleactor)))
        (bind _output_get (set `/Game/Assets/Blueprints/BP_Root.GridCellRef` _outputgridcell _returnvalue_2))
        (`/Game/Assets/Blueprints/Gamemode/GridCell.setRoot` _outputgridcell (`/Game/Assets/Blueprints/Gamemode/GridCell.Type` _output_get) _returnvalue_2)))))

(fn `UpdatePlacement`
  (bind (_worldlocation _worlddirection) (`self.DeprojectMousePositionToWorld`))
  (bind _outhit (`KismetSystemLibrary.LineTraceSingle` _worldlocation (+ _worldlocation (* _worlddirection (10000.0 10000.0 10000.0))) "TraceTypeQuery3"))
  (bind (_bblockinghit _binitialoverlap _time _distance _location) (`GameplayStatics.BreakHitResult` _outhit))
  (if _bblockinghit
    (bind _returnvalue (`GameplayStatics.GetActorOfClass` "/Game/Assets/Blueprints/Gamemode/GridManager.GridManager_C"))
    (bind _outputvector (`/Game/Assets/Blueprints/Gamemode/GridManager.GetClosestGridPos` _returnvalue _location))
    (bind _outputgridcell (`/Game/Assets/Blueprints/Gamemode/GridManager.GetClosestGridCell` _returnvalue _outputvector))
    (if (`/Game/Assets/Blueprints/Gamemode/GridCell.isVisible` _outputgridcell)
      (`self.K2_SetActorLocation` (`self.PlacebleActor`) _outputvector false false))))

(fn `UserConstructionScript`)