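; BP_Root is a spline-based actor that builds spline mesh components in its construction script, one per spline segment.
; Each mesh uses Z as its forward axis and takes local-space tangents from the segment's two spline points.
; Start and end positions come from the PCBP_MouseControls actor rather than the spline, so every segment shares the same endpoints.
; The event graph holds only disabled default events.
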(fn `UserConstructionScript`
  (bind _spline (`self.Spline`))
  (for _index (range (+ (- (`SplineComponent.GetNumberOfSplinePoints` (`self.Spline`)) 2) 1))
    (bind _returnvalue (`AddComponent|NODE_AddSplineMeshComponent-0`))
    (`SplineMeshComponent.SetForwardAxis` _returnvalue "Z" true)
    (bind _returnvalue_2 (`GameplayStatics.GetActorOfClass` "/Game/Assets/Blueprints/Gamemode/PCBP_MouseControls.PCBP_MouseControls_C"))
    (`SplineMeshComponent.SetStartAndEnd` _returnvalue (`/Game/Assets/Blueprints/Gamemode/PCBP_MouseControls.StartPos` _returnvalue_2) (`SplineComponent.GetTangentAtSplinePoint` _spline _index "Local") (`/Game/Assets/Blueprints/Gamemode/PCBP_MouseControls.EndPos` _returnvalue_2) (`SplineComponent.GetTangentAtSplinePoint` _spline (+ _index 1) "Local") true)))