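; AC_PlaceRoot is an actor component that tracks whether its owning actor is in a valid placement and shows the result by color.
; On BeginPlay and whenever the owner begins or ends an overlap, UpdateState sets IsPlacementValid to true only if no actors overlap the owner.
; It then swaps the first material slot on all the owner's static mesh components to Green when valid or Red when blocked.
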(event `self.ReceiveBeginPlay`
  (bind _returnvalue (`self.GetOwner`))
  (add `Actor.OnActorBeginOverlap` _returnvalue (delegate `OverlapStatusChange`))
  (add `Actor.OnActorEndOverlap` _returnvalue (delegate `OverlapStatusChange`))
  (`self.UpdateState`))

(event `OverlapStatusChange`
  (params (OverlappedActor :type "Actor Object Reference") (OtherActor :type "Actor Object Reference"))
  (`self.UpdateState`))

(fn `UpdateState`
  (bind _output_get (set `self.isPlacementValid` (== (`KismetArrayLibrary.Array_Length` (`Actor.GetOverlappingActors` (`self.GetOwner`) "/Script/Engine.Actor")) 0)))
  (for _array_element (`Actor.K2_GetComponentsByClass` (`self.GetOwner`) "/Script/Engine.StaticMeshComponent")
    (if _output_get
      (`PrimitiveComponent.SetMaterial` _array_element 0 "/Game/Assets/Materials/Green.Green")
      (else
        (`PrimitiveComponent.SetMaterial` _array_element 0 "/Game/Assets/Materials/Red.Red")))))