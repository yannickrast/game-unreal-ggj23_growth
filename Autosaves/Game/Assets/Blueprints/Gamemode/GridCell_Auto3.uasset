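; GridCell is a grid tile actor for a root-growing game, with a terrain type and links to its four neighbours.
; On BeginPlay, Poison, Stone and Root cells are flagged as root and non-growable.
; setRoot converts the cell to a root, stores the passed type and actor, then calls Discover on each neighbour.
; Discover swaps the cube's material to match its type and marks it visible.
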(event `self.ReceiveBeginPlay`
  (switch `/Game/Assets/Type` (`self.Type`)
    (:`NewEnumerator2`
      _)
    (:`NewEnumerator3`
      _)
    (:`NewEnumerator4`
      _))
  (set `self.isRoot` true)
  (set `self.isGrowable` false))

(event `setRoot`
  (params (NewParam :type "/Game/Assets/Type Enum" :default "NewEnumerator0") (NewParam2 :type "Actor Object Reference"))
  (set `self.isRoot` true)
  (set `self.Type` NewParam)
  (set `self.NewActor` NewParam2)
  (`self.discover` (`self.NeighbourNorth`))
  (`self.discover` (`self.NeighbourSouth`))
  (`self.discover` (`self.NeighbourEast`))
  (`self.discover` (`self.NeighbourWest`)))

(event `Discover`
  (switch `/Game/Assets/Type` (`self.Type`)
    (:`NewEnumerator0`
      (`PrimitiveComponent.SetMaterial` (`self.Cube`) 0 "/Game/Assets/Materials/M_Ground.M_Ground"))
    (:`NewEnumerator1`
      (`PrimitiveComponent.SetMaterial` (`self.Cube`) 0 "/Game/Assets/Materials/M_Water.M_Water"))
    (:`NewEnumerator2`
      (`PrimitiveComponent.SetMaterial` (`self.Cube`) 0 "/Game/Assets/Materials/M_Poison.M_Poison"))
    (:`NewEnumerator3`
      (`PrimitiveComponent.SetMaterial` (`self.Cube`) 0 "/Game/Assets/Materials/M_Stone.M_Stone"))
    (:`NewEnumerator4`
      (`PrimitiveComponent.SetMaterial` (`self.Cube`) 0 "/Game/Assets/Materials/M_Roots.M_Roots"))
    (:`NewEnumerator5`
      (`PrimitiveComponent.SetMaterial` (`self.Cube`) 0 "/Game/Assets/Materials/M_Mineral.M_Mineral")))
  (set `self.isVisible` true))

(fn `UserConstructionScript`)