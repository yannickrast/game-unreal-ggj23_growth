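; GridManager builds a square grid of GridCell actors on the vertical XZ plane and serves position lookups on it.
; On BeginPlay it spawns the cells, but as wired only one hard-coded cell is made visible and added to GridArray, and type assignments never run.
; It then links north, south, east and west neighbours by index arithmetic.
; Two helpers linearly scan GridArray for the closest cell or its position.
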(event `self.ReceiveBeginPlay`
  (`self.PopulateGrid`)
  (`self.PopulateGridCellNeighbours`))

(fn `GetClosestGridCell`
  (params (inPosition :type "Vector Structure"))
  (returns (outputGridCell :type "/Game/Assets/Blueprints/Gamemode/GridCell Object Reference"))
  (locals (ClosestDistance :type "Float (double-precision)") (ArrayIndex :type Integer))
  (bind _gridarray (`self.GridArray`))
  (set `local.ClosestDistance` (`KismetMathLibrary.Vector_Distance` inPosition (`self.K2_GetActorLocation` (`|GetArrayItem` _gridarray))))
  (for (_array_element _array_index) _gridarray
    (bind _returnvalue (`KismetMathLibrary.Vector_Distance` (`self.K2_GetActorLocation` _array_element) inPosition))
    (if (< _returnvalue (`local.ClosestDistance`))
      (set `local.ClosestDistance` _returnvalue)
      (set `local.ArrayIndex` _array_index)))
  (return (`|GetArrayItem` (`self.GridArray`) (`local.ArrayIndex`))))

(fn `GetClosestGridPos`
  (params (inPosition :type "Vector Structure"))
  (returns (outputVector :type "Vector Structure"))
  (locals (ClosestPos :type "Vector Structure") (ClosestDistance :type "Float (double-precision)"))
  (bind _gridarray (`self.GridArray`))
  (bind _returnvalue (`self.K2_GetActorLocation` (`|GetArrayItem` _gridarray)))
  (set `local.ClosestPos` _returnvalue)
  (set `local.ClosestDistance` (`KismetMathLibrary.Vector_Distance` inPosition _returnvalue))
  (for _array_element _gridarray
    (bind _returnvalue_2 (`self.K2_GetActorLocation` _array_element))
    (bind _returnvalue_3 (`KismetMathLibrary.Vector_Distance` _returnvalue_2 inPosition))
    (if (< _returnvalue_3 (`local.ClosestDistance`))
      (set `local.ClosestPos` _returnvalue_2)
      (set `local.ClosestDistance` _returnvalue_3)))
  (return (`local.ClosestPos`)))

(fn `PopulateGrid`
  (bind _worldgridsize (`self.WorldGridSize`))
  (bind _worldgridsize_2 (`self.WorldGridSize`))
  (bind _worldoffset (`self.WorldOffset`))
  (`KismetArrayLibrary.Array_Clear` (`self.GridArray`))
  (set `self.WorldOffset` (- (* (`KismetMathLibrary.Conv_IntToDouble` (* (`self.GridSize`) _worldgridsize)) 0.5) (* (`KismetMathLibrary.Conv_IntToDouble` _worldgridsize) 0.5)))
  (for _index (range (`self.GridSize`))
    (for _index_2 (range (`self.GridSize`))
      (bind _returnvalue (`|SpawnActorFromClass` "/Game/Assets/Blueprints/Gamemode/GridCell.GridCell_C" (`KismetMathLibrary.MakeTransform` (`KismetMathLibrary.MakeVector` (- (* _index_2 _worldgridsize_2) (+ _worldoffset 300.0)) 0.0 (- (* _worldgridsize_2 _index) (+ _worldoffset 90.0)))) "AlwaysSpawn" "OverrideRootScale" null null))
      (if (and (== _index_2 5) (== _index 10))
        (set `/Game/Assets/Blueprints/Gamemode/GridCell.isVisible` true _returnvalue)
        (`KismetArrayLibrary.Array_Add` (`self.GridArray`) _returnvalue)
        (else
          (switch `int` _index
            (:`0`
              (switch `int` 0
                (:`1`
                  (set `/Game/Assets/Blueprints/Gamemode/GridCell.Type` "NewEnumerator1" _returnvalue))))))))))

(fn `PopulateGridCellNeighbours`
  (bind _gridarray (`self.GridArray`))
  (bind _gridarray_2 (`self.GridArray`))
  (for (_array_element _array_index) (`self.GridArray`)
    (bind _returnvalue (- _array_index (`self.GridSize`)))
    (if (>= _returnvalue 0)
      (set `/Game/Assets/Blueprints/Gamemode/GridCell.NeighbourSouth` (`|GetArrayItem` _gridarray_2 _returnvalue) _array_element))
    (bind _returnvalue_2 (+ _array_index (`self.GridSize`)))
    (if (< _returnvalue_2 (`KismetArrayLibrary.Array_Length` _gridarray_2))
      (set `/Game/Assets/Blueprints/Gamemode/GridCell.NeighbourNorth` (`|GetArrayItem` _gridarray_2 _returnvalue_2) _array_element))
    (if (not (or (== _array_index 0) (== (mod _array_index (`self.GridSize`)) 0)))
      (set `/Game/Assets/Blueprints/Gamemode/GridCell.NeighbourWest` (`|GetArrayItem` _gridarray (- _array_index 1)) _array_element))
    (if (not (== (mod (+ _array_index 1) (`self.GridSize`)) 0))
      (set `/Game/Assets/Blueprints/Gamemode/GridCell.NeighbourEast` (`|GetArrayItem` _gridarray (+ _array_index 1)) _array_element))))

(fn `UserConstructionScript`)