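; GridCell is a grid tile Blueprint with a cell type, four cardinal neighbour references and root, growable and visible state.
; setRoot marks the cell as a root, stores the given type and actor, then calls Debug on its north, south, east and west neighbours.
; Debug switches on type, but every branch applies the Green material to the Cube and sets the cell growable, then it flags the cell visible.
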(event `self.ReceiveBeginPlay`)

(event `setRoot`
  (params (NewParam :type "/Game/Assets/Type Enum" :default "NewEnumerator0") (NewParam2 :type "Actor Object Reference"))
  (set `self.isRoot` true)
  (set `self.Type` NewParam)
  (set `self.NewActor` NewParam2)
  (`self.Debug` (`self.NeighbourNorth`))
  (`self.Debug` (`self.NeighbourSouth`))
  (`self.Debug` (`self.NeighbourEast`))
  (`self.Debug` (`self.NeighbourWest`)))

(event `Debug`
  (switch `/Game/Assets/Type` (`self.Type`)
    (:`NewEnumerator0`
      (`PrimitiveComponent.SetMaterial` (`self.Cube`) 0 "/Game/Assets/Materials/Green.Green")
      (set `self.isGrowable` true))
    (:`NewEnumerator1`
      (`PrimitiveComponent.SetMaterial` (`self.Cube`) 0 "/Game/Assets/Materials/Green.Green")
      (set `self.isGrowable` true))
    (:`NewEnumerator2`
      (`PrimitiveComponent.SetMaterial` (`self.Cube`) 0 "/Game/Assets/Materials/Green.Green")
      (set `self.isGrowable` true))
    (:`NewEnumerator3`
      (`PrimitiveComponent.SetMaterial` (`self.Cube`) 0 "/Game/Assets/Materials/Green.Green")
      (set `self.isGrowable` true))
    (:`NewEnumerator4`
      (`PrimitiveComponent.SetMaterial` (`self.Cube`) 0 "/Game/Assets/Materials/Green.Green")
      (set `self.isGrowable` true))
    (:`NewEnumerator5`
      (`PrimitiveComponent.SetMaterial` (`self.Cube`) 0 "/Game/Assets/Materials/Green.Green")
      (set `self.isGrowable` true)))
  (set `self.isVisible` true))

(fn `UserConstructionScript`)